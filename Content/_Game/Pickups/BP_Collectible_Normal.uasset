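; BP_Collectible_Normal is the basic pickup that the player ball collects by touching it.
; When the player pawn overlaps its Box, it increments CollectibleNormalCount on the BallPlayerState.
; It then plays a pickup sound, spawns a burst effect at its location and destroys itself.
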(event `self.Box.OnComponentBeginOverlap`
  (params (OverlappedComponent :type "PrimitiveComponent Object Reference") (OtherActor :type "Actor Object Reference") (OtherComp :type "PrimitiveComponent Object Reference") (OtherBodyIndex :type Integer) (bFromSweep :type Boolean) (SweepResult :type "HitResult Structure (by ref)"))
  (if (== OtherActor (`GameplayStatics.GetPlayerPawn` 0))
    (bind _asball_player_state (cast `/Game/_Game/BallGame/BallPlayerState` (`GameplayStatics.GetPlayerState` 0)))
    (set `/Game/_Game/BallGame/BallPlayerState.CollectibleNormalCount` (+ (`/Game/_Game/BallGame/BallPlayerState.CollectibleNormalCount` _asball_player_state) 1) _asball_player_state)
    (`GameplayStatics.PlaySoundAtLocation` "/Game/_Game/Audio/NormalPickup_Cue.NormalPickup_Cue" (`self.K2_GetActorLocation`) (struct) 1.0 1.0 0.0 null null null null)
    (`NiagaraFunctionLibrary.SpawnSystemAtLocation` "/Game/_Game/Particles/PS_NormalBurst.PS_NormalBurst" (`self.K2_GetActorLocation`))
    (`self.K2_DestroyActor`)))

(fn `UserConstructionScript`)