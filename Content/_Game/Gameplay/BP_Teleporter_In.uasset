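; BP_Teleporter_In is a teleporter entrance that moves the player pawn to the location of a referenced TeleportLocation actor.
; When the player pawn overlaps its Box, it plays an entry sound and particle system, disables input and waits briefly.
; It then moves the pawn without sweeping, plays exit sound and effects at the destination, and re-enables input.
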(event `self.Box.OnComponentBeginOverlap`
  (params (OverlappedComponent :type "PrimitiveComponent Object Reference") (OtherActor :type "Actor Object Reference") (OtherComp :type "PrimitiveComponent Object Reference") (OtherBodyIndex :type Integer) (bFromSweep :type Boolean) (SweepResult :type "HitResult Structure (by ref)"))
  (bind _returnvalue (`self.K2_GetActorLocation` (`self.TeleportLocation`)))
  (if (== OtherActor (`GameplayStatics.GetPlayerPawn` 0))
    (`GameplayStatics.PlaySound2D` "/Game/_Game/Audio/Teleport_In.Teleport_In" 1.0 1.0 0.0 null null)
    (`NiagaraFunctionLibrary.SpawnSystemAtLocation` "/Game/_Game/Particles/PS_Teleport_IN.PS_Teleport_IN" (`SceneComponent.K2_GetComponentLocation` (`self.Box`)))
    (`self.DisableInput` (`GameplayStatics.GetPlayerPawn` 0) (`GameplayStatics.GetPlayerController` 0))
    (`KismetSystemLibrary.Delay` 1.0)
    (`self.K2_SetActorLocation` (`GameplayStatics.GetPlayerPawn` 0) _returnvalue false false)
    (`GameplayStatics.PlaySound2D` "/Game/_Game/Audio/Teleport_Out.Teleport_Out" 1.0 1.0 0.0 null null)
    (`NiagaraFunctionLibrary.SpawnSystemAtLocation` "/Game/_Game/Particles/PS_Teleport_Out.PS_Teleport_Out" _returnvalue)
    (`self.EnableInput` (`GameplayStatics.GetPlayerPawn` 0) (`GameplayStatics.GetPlayerController` 0))))

(fn `UserConstructionScript`)