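; BP_CheckPoint is a checkpoint actor that records a new respawn location for the ball player.
; When the first player's pawn overlaps its Box, it spawns a Niagara effect at its SpawnPoint component and plays a checkpoint sound.
; It then writes the SpawnPoint world transform into that player's BallPlayerState.
; Nothing disables the trigger, so each re-entry repeats the effect, sound and update.
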(event `self.Box.OnComponentBeginOverlap`
  (params (OverlappedComponent :type "PrimitiveComponent Object Reference") (OtherActor :type "Actor Object Reference") (OtherComp :type "PrimitiveComponent Object Reference") (OtherBodyIndex :type Integer) (bFromSweep :type Boolean) (SweepResult :type "HitResult Structure (by ref)"))
  (if (== OtherActor (`GameplayStatics.GetPlayerPawn` 0))
    (`NiagaraFunctionLibrary.SpawnSystemAtLocation` "/Game/_Game/Particles/PS_CheckPoint.PS_CheckPoint" (`SceneComponent.K2_GetComponentLocation` (`self.SpawnPoint`)))
    (`GameplayStatics.PlaySound2D` "/Game/_Game/Audio/CheckPoint.CheckPoint" 1.0 1.0 0.0 null null)
    (bind _asball_player_state (cast `/Game/_Game/BallGame/BallPlayerState` (`GameplayStatics.GetPlayerState` 0)))
    (set `/Game/_Game/BallGame/BallPlayerState.SpawnPoint` (`SceneComponent.K2_GetComponentToWorld` (`self.SpawnPoint`)) _asball_player_state)))

(fn `UserConstructionScript`)